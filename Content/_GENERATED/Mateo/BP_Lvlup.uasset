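; BP_Lvlup is an actor that simulates a simple experience and level-up loop on a timer, with no player input.
; BeginPlay starts a looping timer at the Tiempo interval that fires SubirDeNivel, which adds fixed experience through SumarExperiencia and prints the total.
; When Experiencia reaches its threshold, Nivel increments and experience resets to zero; the actor destroys itself upon reaching level 5.
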(event `self.ReceiveBeginPlay`
  (`KismetSystemLibrary.K2_SetTimerDelegate` (delegate `SubirDeNivel`) (`self.Tiempo`) true))

(event `SubirDeNivel`
  (`self.SumarExperiencia` 50)
  (`KismetSystemLibrary.PrintString` (`KismetStringLibrary.Concat_StrStr` "Experiencia adquirida! \n" (`KismetStringLibrary.Conv_IntToString` (`self.Experiencia`))))
  (if (>= (`self.Experiencia`) 100)
    (set `self.Nivel` (+ (`self.Nivel`) 1))
    (set `self.Experiencia` 0)
    (if (== (`self.Nivel`) 5)
      (`self.K2_DestroyActor`))))

(fn `SumarExperiencia`
  (params (Exp :type Integer))
  (locals (NewLocalVar :type Integer :default 0))
  (set `self.Experiencia` (+ Exp (`self.Experiencia`))))

(fn `UserConstructionScript`)