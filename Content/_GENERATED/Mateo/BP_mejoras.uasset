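; BP_mejoras is an upgrade ("mejoras") test Blueprint that reports boosted damage and speed values on BeginPlay.
; Nested branches on Potencia and Rapida print doubled damage, then doubled speed, then both quadrupled when both flags are set.
; Rapida is only checked when Potencia is true, so a speed-only upgrade prints nothing.
; Multipliers affect only the printed text, as Daño and Velocidad are reassigned their own values.
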(event `self.ReceiveBeginPlay`
  (if (`self.bPotencia`)
    (bind _output_get (set `self.Daño` (`self.Daño`)))
    (`KismetSystemLibrary.PrintString` (`KismetStringLibrary.Concat_StrStr` "Mi daño es: \n" (`KismetStringLibrary.Conv_DoubleToString` (* _output_get 2.0))))
    (if (`self.bRapida`)
      (bind _output_get_2 (set `self.Velocidad` (`self.Velocidad`)))
      (`KismetSystemLibrary.PrintString` (`KismetStringLibrary.Concat_StrStr` "Mi velocidad es: \n" (`KismetStringLibrary.Conv_DoubleToString` (* _output_get_2 2.0))))
      (if (and (`self.bRapida`) (`self.bPotencia`))
        (bind _output_get_3 (set `self.Daño` (`self.Daño`)))
        (bind _output_get_4 (set `self.Velocidad` (`self.Velocidad`)))
        (`KismetSystemLibrary.PrintString` (`KismetStringLibrary.Concat_StrStr` "Mi velocidad es: \n" (`KismetStringLibrary.Conv_DoubleToString` (* _output_get_4 4.0)) " \nMi daño es: \n" (`KismetStringLibrary.Conv_DoubleToString` (* _output_get_3 4.0))))))))

(fn `UserConstructionScript`)